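; BP_AmmoBox is an ammo pickup whose lid pops off when it is picked up.
; The box stays static, and the lid ignores Pawn collision.
; Detection highlights the lid through custom depth until it has detached.
; PickUp enables lid physics, fires a radial impulse, detaches the lid and sends the AddAmmos message to the owner.
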(event EventBeginPlay
  (|CallParentFunction)
  (Collision|SetCollisionResponsetoChannel (Variables|Default|GetLidMesh) "ECC_Pawn" "ECR_Ignore")
  (Physics|SetSimulatePhysics (Variables|Default|GetStaticMeshComponent) false))

(event Collision|EventActorBeginOverlap
  (params (OtherActor :type Actor%20Object%20Reference))
  (|CallParentFunction OtherActor) ; This node is disabled and will not be called.\nDrag off pins to build functionality.
)

(event EventTick
  (params (DeltaSeconds :type Float%20%28single-precision%29))
  (|CallParentFunction DeltaSeconds) ; This node is disabled and will not be called.\nDrag off pins to build functionality.
)

(event EventPickUp
  (params (Owner :type Pawn%20Object%20Reference))
  (Physics|SetSimulatePhysics (Variables|Default|GetLidMesh) true)
  (Class|RadialForceComponent|FireImpulse (Variables|Default|GetRadialForce))
  (Transformation|DetachFromComponent (Variables|Default|GetLidMesh) "KeepWorld" "KeepWorld" "KeepWorld" true)
  (Variables|Default|SetDetached true)
  (Class|IPlayerAttrs|AddAmmos(Message) Owner))

(event EventOnDetected
  (params (Owner :type Pawn%20Object%20Reference) (Active :type Boolean))
  (|CallParentFunction Owner Active)
  (Rendering|SetRenderCustomDepth (Variables|Default|GetLidMesh) (and (not (Variables|Default|GetDetached)) Active)))

(fn ConstructionScript
  (|CallParentFunction))
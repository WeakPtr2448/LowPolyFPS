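; BP_HeadSet is a headset item that can be picked up and worn by its owner.
; Its PickUp event finds the owner's first static mesh component tagged "HeadSet" and copies the item's mesh onto it.
; The world actor then destroys itself, so the pickup works as a mesh swap rather than an attachment.
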(event EventBeginPlay
  (|CallParentFunction) ; This node is disabled and will not be called.\nDrag off pins to build functionality.
)

(event Collision|EventActorBeginOverlap
  (params (OtherActor :type Actor%20Object%20Reference))
  (|CallParentFunction OtherActor) ; This node is disabled and will not be called.\nDrag off pins to build functionality.
)

(event EventTick
  (params (DeltaSeconds :type Float%20%28single-precision%29))
  (|CallParentFunction DeltaSeconds) ; This node is disabled and will not be called.\nDrag off pins to build functionality.
)

(event EventPickUp
  (params (Owner :type Pawn%20Object%20Reference))
  (Components|StaticMesh|SetStaticMesh (Utilities|Array|Get(acopy) (Actor|GetComponentsbyTag Owner "/Script/Engine.StaticMeshComponent" "HeadSet")) (Variables|/Script/Engine.StaticMeshComponent|GetStaticMesh (Variables|Default|GetStaticMeshComponent)))
  (Actor|DestroyActor))

(fn ConstructionScript
  (|CallParentFunction))
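; BP_Hook is the projectile actor of the grapple hook, launched with a given velocity.
; On BeginPlay it applies InVelocity to its ProjectileMovement component and records its spawn location.
; Each tick it measures the distance from that location and destroys itself once it exceeds a fixed maximum range.
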(event EventBeginPlay
  (Variables|/Script/Engine.MovementComponent|SetVelocity (Variables|Default|GetProjectileMovement) (Variables|Default|GetInVelocity))
  (Variables|Default|SetInitLocation (Transformation|GetActorLocation)))

(event EventTick
  (params (DeltaSeconds :type Float%20%28single-precision%29))
  (if (> (Math|Vector|Distance(Vector) (Transformation|GetActorLocation) (Variables|Default|GetInitLocation)) 5e+03)
    (Actor|DestroyActor)))

(fn ConstructionScript)
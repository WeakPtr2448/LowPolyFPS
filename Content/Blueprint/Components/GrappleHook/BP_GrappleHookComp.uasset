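; Grappling hook component that pulls its owning character toward wherever the fired hook hits.
; Firing spawns a moving hook actor and a cable linking it to the character.
; A hit removes gravity and ground friction, changes air control and launches the character, while Tick adds force toward the hook.
; Moving away, getting close or passing the hook destroys it, and its destroyed event removes the cable and restores cached movement settings.
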(event Custom|Initialize
  (params (OwningCharacter :type Character%20Object%20Reference))
  (bind _output_get (Variables|Default|SetOwning%20Character OwningCharacter))
  (bind _output_get_2 (Variables|Default|SetCharacter%20Movement (Variables|/Script/Engine.Character|GetCharacterMovement _output_get)))
  (Variables|Default|SetDefaultGravity%20Scale (Variables|/Script/Engine.CharacterMovementComponent|GetGravityScale _output_get_2))
  (Variables|Default|SetDefaultGround%20Friction (Variables|/Script/Engine.CharacterMovementComponent|GetGroundFriction _output_get_2))
  (Variables|Default|SetDefaultAir%20Control (Variables|/Script/Engine.CharacterMovementComponent|GetAirControl _output_get_2)))

(event EventBeginPlay)

(event EventTick
  (params (DeltaSeconds :type Float%20%28single-precision%29))
  (switch Utilities|FlowControl|Switch|SwitchonE_GrappleState (Variables|Default|GetGrappleState)
    (:NewEnumerator2
      (Physics|AddForce (Variables|Default|GetCharacter%20Movement) (* (Utilities|ToGrappleHookDir) 5e+01))
      (if (< (Math|Vector|DotProduct (Utilities|ToGrappleHookDir) (Math|Vector|Normalize (Transformation|GetVelocity (Variables|Default|GetOwning%20Character)))) 0.0)
        (CallFunction|CancleGrappleHook)
        (elif (<= (Math|Vector|Distance(Vector) (Transformation|GetActorLocation (Variables|Default|GetHook)) (Transformation|GetActorLocation (Variables|Default|GetOwning%20Character))) 3e+02)
          (CallFunction|CancleGrappleHook)
          (elif (< (Math|Vector|DotProduct (Variables|Default|GetInitialDir) (Utilities|ToGrappleHookDir)) 0.0)
            (CallFunction|CancleGrappleHook)))))))

(fn FireGrappleHook
  (params (TargetLocation :type Vector) (Offset :type Vector))
  (bind _returnvalue (Utilities|GetFireLocation Offset))
  (bind _returnvalue_2 (- TargetLocation _returnvalue))
  (bind _returnvalue_3 (Math|Vector|Normalize _returnvalue_2))
  (Variables|Default|SetGrappleState "NewEnumerator1")
  (bind _returnvalue_4 (Game|SpawnActorfromClass "/Game/Blueprint/Components/GrappleHook/BP_Hook.BP_Hook_C" (Math|Transform|MakeTransform _returnvalue (Math|Conversions|RotationFromXVector _returnvalue_3) "0.100000,0.100000,0.100000") "Undefined" 0 (* _returnvalue_3 (Variables|Default|GetHookSpeed)) 0))
  (bind _output_get (Variables|Default|SetHook _returnvalue_4))
  (Collision|BindEventtoOnActorHit _output_get (EventDispatchers|CreateEvent :!event OnGrappleHookHit))
  (Game|BindEventtoOnDestroyed _output_get (EventDispatchers|CreateEvent :!event OnGrappleHookDestroyed))
  (bind _returnvalue_5 (Game|SpawnActorfromClass "/Game/Blueprint/Components/GrappleHook/BP_GrappleCable.BP_GrappleCable_C" (Math|Transform|MakeTransform (Utilities|GetFireLocation Offset) (Math|Conversions|RotationFromXVector (Utilities|ToGrappleHookDir)) "0.500000,0.500000,0.500000") "Undefined" 0 0))
  (bind _output_get_2 (Variables|Default|SetGrappleCable _returnvalue_5))
  (Transformation|AttachActorToActor _output_get_2 (Variables|Default|GetOwning%20Character) "None" "KeepWorld" "KeepWorld" "KeepWorld" true)
  (Class|CableComponent|SetAttachEndto (Variables|/Script/CableComponent.CableActor|GetCableComponent _output_get_2) (Variables|Default|GetHook) "None" "None"))

(fn CancleGrappleHook
  (bind _hook (Variables|Default|GetHook)
    (:then
      (Actor|DestroyActor _hook)
      (Variables|Default|SetHook 0))
    (:else)))

(fn OnGrappleHookHit
  (params (SelfActor :type Actor%20Object%20Reference) (OtherActor :type Actor%20Object%20Reference) (NormalImpulse :type Vector) (Hit :type Hit%20Result%20Structure%20%28by%20ref%29))
  (bind _dir (Utilities|ToGrappleHookDir))
  (bind _character_movement (Variables|Default|GetCharacter%20Movement))
  (bind (_x _y) (Math|Vector|BreakVector _dir))
  (Variables|Default|SetGrappleState "NewEnumerator2")
  (Variables|/Script/Engine.CharacterMovementComponent|SetGravityScale _character_movement 0.0)
  (Variables|/Script/Engine.CharacterMovementComponent|SetGroundFriction _character_movement 0.0)
  (Variables|/Script/Engine.CharacterMovementComponent|SetAirControl _character_movement 0.6)
  (Variables|/Script/Engine.MovementComponent|SetVelocity (Variables|Default|GetCharacter%20Movement) (* (Utilities|ToGrappleHookDir) 2.5e+03))
  (Variables|Default|SetInitialDir (Math|Vector|MakeVector _x _y 0.0))
  (return))

(fn OnGrappleHookDestroyed
  (params (DestroyedActor :type Actor%20Object%20Reference))
  (bind _character_movement (Variables|Default|GetCharacter%20Movement))
  (Variables|Default|SetGrappleState "NewEnumerator0")
  (Utilities|FlowControl|Sequence
    (:then_0
      (bind _grapplecable (Variables|Default|GetGrappleCable)
        (:then
          (Actor|DestroyActor _grapplecable)
          (Variables|Default|SetGrappleCable 0))
        (:else)))
    (:then_1
      (Variables|/Script/Engine.CharacterMovementComponent|SetGravityScale _character_movement (Variables|Default|GetDefaultGravity%20Scale))
      (Variables|/Script/Engine.CharacterMovementComponent|SetGroundFriction _character_movement (Variables|Default|GetDefaultGround%20Friction))
      (Variables|/Script/Engine.CharacterMovementComponent|SetAirControl _character_movement (Variables|Default|GetDefaultAir%20Control)))))
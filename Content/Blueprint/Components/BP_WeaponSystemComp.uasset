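; Weapon component that handles firing, recoil, effects and reload ammo math for rifles, handguns, SMGs and single-reload shotguns.
; TryStartFire runs FireLogic with a looping timer for auto or cooldown for semi, and requests a reload when empty.
; Each shot applies curve-driven recoil that sets projectile spread, then spawns bullets, montages, effects, sound and casings, with shotgun multi-pellets and bolt animation.
; Weapon data and ammo pass through messages to the owning weapon and character.
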(event EventBeginPlay)

(fn Initialize
  (params (FireDuration :type Float%20%28single-precision%29) (bAuto :type Boolean))
  (Variables|Default|SetFireDuration FireDuration)
  (Variables|Default|SetbAuto bAuto))

(fn SpawnBullets
  (bind _returnvalue (Components|GetOwner))
  (bind _spreadvalue (Variables|Default|GetSpreadValue))
  (bind _weaponattr (Class|IWeaponAttrs|GetWeaponAttrs(Message) (Components|GetOwner)))
  (bind _weaponmesh (Class|IWeaponAttrs|GetWeaponMesh(Message) (Components|GetOwner)))
  (bind _asplayer_controller (Utilities|Casting|CastToPlayerController (Pawn|GetController (CallFunction|GetOwningCharacter))))
  (for _index (range 0 (Utilities|Select :Index (.WeaponType (Utilities|Struct|BreakS_WeaponAttrs _weaponattr)) :NewEnumerator0 0 :NewEnumerator1 0 :NewEnumerator3 0 :NewEnumerator5 8))
    (bind _returnvalue_2 (Game|SpawnActorfromClass (.AmmoClass (Utilities|Struct|BreakS_WeaponAttrs _weaponattr)) (Math|Transform|MakeTransform (Transformation|GetSocketLocation _weaponmesh (Variables|Default|GetMuzzleSocket)) (Math|Conversions|RotationFromXVector (Class|KismetMathLibrary|RandomUnitVectorinEllipticalConeinRadians (- (.TargetLocation (CallFunction|GetTargetLocation _asplayer_controller 1e+04 "TraceTypeQuery1")) (Transformation|GetSocketLocation _weaponmesh (Variables|Default|GetMuzzleSocket))) (* _spreadvalue (.X (Math|Vector2D|BreakVector2D (Utilities|Struct|BreakS_Recoil (.Recoil (Utilities|Struct|BreakS_WeaponAttrs _weaponattr)))))) (* _spreadvalue (.Y (Math|Vector2D|BreakVector2D (Utilities|Struct|BreakS_Recoil (.Recoil (Utilities|Struct|BreakS_WeaponAttrs _weaponattr)))))))) "2.000000,2.000000,2.000000") "Undefined" (Components|GetOwner) (CallFunction|GetOwningCharacter)))
    (Default|Initialize _returnvalue_2 (Class|KismetMathLibrary|RandomUnitVectorinEllipticalConeinRadians (- (.TargetLocation (CallFunction|GetTargetLocation _asplayer_controller 1e+04 "TraceTypeQuery1")) (Transformation|GetSocketLocation _weaponmesh (Variables|Default|GetMuzzleSocket))) (* _spreadvalue (.X (Math|Vector2D|BreakVector2D (Utilities|Struct|BreakS_Recoil (.Recoil (Utilities|Struct|BreakS_WeaponAttrs _weaponattr)))))) (* _spreadvalue (.Y (Math|Vector2D|BreakVector2D (Utilities|Struct|BreakS_Recoil (.Recoil (Utilities|Struct|BreakS_WeaponAttrs _weaponattr))))))) (Utilities|Select :Index (.AmmoType (Utilities|Struct|BreakS_WeaponAttrs _weaponattr)) :NewEnumerator0 0.0 :NewEnumerator1 8e+03 :NewEnumerator6 8.5e+03 :NewEnumerator3 1e+04 :NewEnumerator5 5e+02)))
  (bind (_currentammo _maxammo) (Class|IWeaponAttrs|GetAmmos(Message) _returnvalue))
  (Class|IWeaponAttrs|SetAmmos(Message) _returnvalue (- _currentammo 1) _maxammo)
  (Utilities|HasAmmo
    (:false
      (Class|IWeaponAttrs|SetSlideBack(Message) (Components|GetOwner) false))))

(fn GetOwningCharacter
  (bind _aspawn (Utilities|Casting|CastToPawn (Components|GetOwner (Components|GetOwner))))
  (return _aspawn))

(fn PlayCharacterAnim
  (bind _owningpawn (CallFunction|GetOwningCharacter))
  (bind _characteranims (Class|IPlayerAttrs|GetCharacterAnims(Message) _owningpawn))
  (bind _montagelength (Class|IPlayerAttrs|PlayCharacterAnimMontage(Message) _owningpawn (.Fire (Utilities|Struct|BreakS_CharacterAnims _characteranims))))
  (return _montagelength))

(fn PlayWeaponAnim
  (bind _returnvalue (Components|GetOwner))
  (bind _weaponmesh (Class|IWeaponAttrs|GetWeaponMesh(Message) _returnvalue))
  (bind _weaponanims (Class|IWeaponAttrs|GetWeaponAnims(Message) _returnvalue))
  (Animation|Montage|MontagePlay (Components|SkeletalMesh|GetAnimInstance _weaponmesh) (.Fire (Utilities|Struct|BreakS_WeaponAnims _weaponanims)) 1.0 "MontageLength" 0.0 true))

(fn FireEffect
  ;[1 1 1] 开火特效
  (bind _weaponattr (Class|IWeaponAttrs|GetWeaponAttrs(Message) (Components|GetOwner)))
  (bind _weaponmesh (Class|IWeaponAttrs|GetWeaponMesh(Message) (Components|GetOwner)))
  (Effects|SpawnEmitterAttached (select (Utilities|GetHasSilencer) (.FireSuppressedEffect (Utilities|Struct|BreakS_WeaponAttrs _weaponattr)) (.FireEffect (Utilities|Struct|BreakS_WeaponAttrs _weaponattr))) _weaponmesh (Variables|Default|GetMuzzleSocket) (Math|Vector|MakeVector (.X (Math|Vector|BreakVector (.location (Transformation|GetSocketTransform _weaponmesh (Variables|Default|GetMuzzleSocket) "RTS_Component")))) (- (.Y (Math|Vector|BreakVector (.location (Transformation|GetSocketTransform _weaponmesh (Variables|Default|GetMuzzleSocket) "RTS_Component")))) 18.0) (- (.Z (Math|Vector|BreakVector (.location (Transformation|GetSocketTransform _weaponmesh (Variables|Default|GetMuzzleSocket) "RTS_Component")))) 6.0)) (Math|Rotator|MakeRotator (.Roll (Math|Rotator|BreakRotator (.rotation (Transformation|GetSocketTransform _weaponmesh (Variables|Default|GetMuzzleSocket) "RTS_Component")))) (.Pitch (Math|Rotator|BreakRotator (.rotation (Transformation|GetSocketTransform _weaponmesh (Variables|Default|GetMuzzleSocket) "RTS_Component")))) (+ (.Yaw (Math|Rotator|BreakRotator (.rotation (Transformation|GetSocketTransform _weaponmesh (Variables|Default|GetMuzzleSocket) "RTS_Component")))) 9e+01))))

(fn StopFireEffect
  (if (> (Variables|Default|GetShotAmmo) 10)
    (bind _weaponmesh (Class|IWeaponAttrs|GetWeaponMesh(Message) (Components|GetOwner)))
    (Effects|SpawnEmitterAttached "/Game/LowPolyShooterPack/Art/Effects/Particles/PS_Muzzle_Smoke.PS_Muzzle_Smoke" _weaponmesh (Variables|Default|GetMuzzleSocket) "0, 0, 0" "0, 0, 0" "1.000000,1.000000,1.000000" "SnapToTarget")))

(fn PlayFireSound
  (bind _returnvalue (Components|GetOwner))
  (bind _weaponattr (Class|IWeaponAttrs|GetWeaponAttrs(Message) _returnvalue))
  (Audio|PlaySoundatLocation (select (Utilities|GetHasSilencer) (.FireSupressed (Utilities|Struct|BreakS_WeaponSounds (.FireSound (Utilities|Struct|BreakS_WeaponAttrs _weaponattr)))) (.FireNormal (Utilities|Struct|BreakS_WeaponSounds (.FireSound (Utilities|Struct|BreakS_WeaponAttrs _weaponattr))))) (Transformation|GetActorLocation _returnvalue) "0, 0, 0" 1.0 1.0 0.0 0 0 0))

(fn SpawnEject
  (bind _returnvalue (Components|GetOwner))
  (bind _maxammo (Class|IWeaponAttrs|GetAmmos(Message) (Components|GetOwner)))
  (if (> _maxammo 0)
    (bind _weaponattr (Class|IWeaponAttrs|GetWeaponAttrs(Message) _returnvalue))
    (bind _weaponmesh (Class|IWeaponAttrs|GetWeaponMesh(Message) _returnvalue))
    (bind _returnvalue_2 (Game|SpawnActorfromClass (Utilities|Struct|BreakS_WeaponAttrs _weaponattr) (Math|Transform|MakeTransform (.location (Transformation|GetSocketTransform _weaponmesh (Variables|Default|GetEjectSocket) "RTS_World")) (.rotation (Transformation|GetSocketTransform _weaponmesh (Variables|Default|GetEjectSocket) "RTS_World")) "1,1,1") "Undefined" 0 0))
    (Default|LaunchEject _returnvalue_2 (* (Math|Rotator|GetRotationXVector (.rotation (Transformation|GetSocketTransform _weaponmesh (Variables|Default|GetEjectSocket) "RTS_World"))) (Math|Random|RandomFloatinRange 1.5e+02 2e+02)))))

(fn ReloadLogic
  (bind (_currentammo _maxammo _standardammo) (Class|IWeaponAttrs|GetAmmos(Message) (Components|GetOwner)))
  (LocalVariables|SetCurrentAmmo _currentammo)
  (LocalVariables|SetStandardAmmo _standardammo)
  (LocalVariables|SetMaxAmmo _maxammo)
  (if (> (LocalVariables|GetMaxAmmo) 0)
    (bind _weaponattr (Class|IWeaponAttrs|GetWeaponAttrs(Message) (Components|GetOwner)))
    (switch Utilities|FlowControl|Switch|SwitchonE_WeaponType (.WeaponType (Utilities|Struct|BreakS_WeaponAttrs _weaponattr))
      (:NewEnumerator0
        (LocalVariables|SetLostAmmo (- (LocalVariables|GetStandardAmmo) (LocalVariables|GetCurrentAmmo)) :!label _label)
        (if (> (LocalVariables|GetLostAmmo) (LocalVariables|GetMaxAmmo))
          (LocalVariables|SetCurrentAmmo (+ (LocalVariables|GetCurrentAmmo) (LocalVariables|GetMaxAmmo)))
          (LocalVariables|SetMaxAmmo 0)
          (else
            (LocalVariables|SetCurrentAmmo (LocalVariables|GetStandardAmmo))
            (LocalVariables|SetMaxAmmo (- (LocalVariables|GetMaxAmmo) (LocalVariables|GetLostAmmo)))))
        (Class|IWeaponAttrs|SetAmmos(Message) (Components|GetOwner) (LocalVariables|GetCurrentAmmo) (LocalVariables|GetMaxAmmo)))
      (:NewEnumerator1
        (goto _label))
      (:NewEnumerator3
        (goto _label))
      (:NewEnumerator5
        ;[1 1 1] SingleReload
        (Math|Integer|IncrementInt (LocalVariables|GetCurrentAmmo)
          (:%20%20
            (Math|Integer|DecrementInt (LocalVariables|GetMaxAmmo)
              (:%20%20
                (Class|IWeaponAttrs|SetAmmos(Message) (Components|GetOwner) (LocalVariables|GetCurrentAmmo) (LocalVariables|GetMaxAmmo))))))))))

(fn Recoil
  (bind _weaponattr (Class|IWeaponAttrs|GetWeaponAttrs(Message) (Components|GetOwner)))
  (Variables|Default|SetRecoilValue (Math|Curves|GetFloatValue (.RecoilCurve (Utilities|Struct|BreakS_Recoil (.Recoil (Utilities|Struct|BreakS_WeaponAttrs _weaponattr)))) (/ (Math|Conversions|ToFloat(Integer) (Variables|Default|GetShotAmmo)) (Math|Conversions|ToFloat(Integer) (.StandardAmmo (Utilities|Struct|BreakS_WeaponAttrs _weaponattr))))))
  (bind _aimkeydown (Utilities|GetIsAimming))
  (Pawn|Input|AddControllerPitchInput (CallFunction|GetOwningCharacter) (* (+ (* (select _aimkeydown 0.3 1.0) (* (Variables|Default|GetRecoilValue) (.X (Math|Vector2D|BreakVector2D (.RecoilValue (Utilities|Struct|BreakS_Recoil (.Recoil (Utilities|Struct|BreakS_WeaponAttrs _weaponattr)))))))) (select (Utilities|GetIsMoving) 1.0 0.0)) -0.1))
  (Variables|Default|SetSpreadValue (* (+ (* (select _aimkeydown 0.3 1.0) (* (Variables|Default|GetRecoilValue) (.X (Math|Vector2D|BreakVector2D (.RecoilValue (Utilities|Struct|BreakS_Recoil (.Recoil (Utilities|Struct|BreakS_WeaponAttrs _weaponattr)))))))) (select (Utilities|GetIsMoving) 1.0 0.0)) 0.01)))

(fn FireCoolDown
  ;[0.3229 1 0.8392] 下一次开火的冷却（仅单发开火模式）
  (if (not (Variables|Default|GetbAuto))
    (bind _returnvalue (Utilities|Time|SetTimerbyEvent (EventDispatchers|CreateEvent :!event Custom|FireCoolDownTime) (Variables|Default|GetFireDuration)))
    (Variables|Default|SetCoolDownTimerHandle _returnvalue)))

(event Custom|TryStartFire
  (if (Variables|Default|GetbCanFire)
    (Utilities|HasAmmo
      (:true
        (Utilities|FlowControl|Sequence
          (:then_0
            (CallFunction|FireLogic)
            (if (Variables|Default|GetbAuto)
              (bind _returnvalue (Utilities|Time|SetTimerbyEvent (EventDispatchers|CreateEvent :!event Custom|FireLogic) (Variables|Default|GetFireDuration) (Variables|Default|GetbAuto)))
              (Variables|Default|SetFireTimerHandle _returnvalue)
              (else
                (Variables|Default|SetbCanFire false))))))
      (:false
        ;[1 1 1] 自动换弹
        (Class|IWeaponAttrs|SetSlideBack(Message) (Components|GetOwner) false)
        (Class|IPlayerAttrs|PlayCharacterAnimMontage(Message) (CallFunction|GetOwningCharacter) "/Game/LowPolyShooterPack/Art/Characters/Animations/_Common/AM_FP_PCH_Fire_Empty.AM_FP_PCH_Fire_Empty")
        (Utilities|FlowControl|RetriggerableDelay 0.25)
        (Class|IPlayerAttrs|CallReloadEvent(Message) (CallFunction|GetOwningCharacter))))))

(event Custom|TryStopFire
  (Utilities|Time|ClearandInvalidateTimerbyHandle (Variables|Default|GetFireTimerHandle))
  (Fire|StopFireEffect)
  (Variables|Default|SetShotAmmo 0))

(event Custom|FireLogic
  (bind _owningpawn (CallFunction|GetOwningCharacter))
  (bind _returnvalue (Components|GetOwner))
  ;[1 0.5781 0.5781] 开火逻辑
  (Utilities|HasAmmo
    (:true
      (Math|Integer|IncrementInt (Variables|Default|GetShotAmmo)
        (:%20%20
          (Fire|Recoil)
          (Fire|SpawnBullets)
          (bind _length (Fire|PlayCharacterAnim))
          (Fire|PlayWeaponAnim)
          (Fire|FireEffect)
          (Class|IPlayerAttrs|CallonUpdateWeaponAmmos(Message) (CallFunction|GetOwningCharacter))
          (Class|IWeaponAttrs|CallUpdateAmmoVisible(Message) (Components|GetOwner))
          ;[1 1 1] 下一次开火冷却
          (Fire|FireCoolDown)
          ;[0.5166 1 0] 播放开火声音
          (Fire|PlayFireSound)
          (bind _weaponattr (Class|IWeaponAttrs|GetWeaponAttrs(Message) (Components|GetOwner)))
          (switch Utilities|FlowControl|Switch|SwitchonE_WeaponType (Utilities|Struct|BreakS_WeaponAttrs _weaponattr)
            (:NewEnumerator0
              (Fire|SpawnEject :!label _label))
            (:NewEnumerator1
              (goto _label))
            (:NewEnumerator3
              (goto _label))
            (:NewEnumerator5
              (bind _currentammo (Class|IWeaponAttrs|GetAmmos(Message) (Components|GetOwner)))
              (if (> _currentammo 0)
                (Utilities|FlowControl|Delay (- _length 0.8))
                (bind _characteranims (Class|IPlayerAttrs|GetCharacterAnims(Message) _owningpawn))
                (Class|IPlayerAttrs|PlayCharacterAnimMontage(Message) _owningpawn (Utilities|Struct|BreakS_CharacterAnims _characteranims))
                (bind _weaponmesh (Class|IWeaponAttrs|GetWeaponMesh(Message) _returnvalue))
                (bind _weaponanims (Class|IWeaponAttrs|GetWeaponAnims(Message) _returnvalue))
                (Animation|Montage|PlayMontage _weaponmesh (Utilities|Struct|BreakS_WeaponAnims _weaponanims)
                  (:then
                    (CallFunction|TryStopFire)))
                (else
                  (CallFunction|TryStopFire))))))))
    (:false
      (CallFunction|TryStopFire))))

(event Custom|FireCoolDownTime
  (Variables|Default|SetbCanFire true)
  (Utilities|Time|ClearandInvalidateTimerbyHandle (Variables|Default|GetCoolDownTimerHandle)))

(event EventTick
  (params (DeltaSeconds :type Float%20%28single-precision%29)))
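; BP_PC is the player controller that manages the main HUD, weapon bag and gunsmith screens.
; It fades the camera in on BeginPlay, adds the HUD on possess and removes it on unpossess.
; Input actions create or remove the bag and gunsmith widgets, switching input mode and cursor, with gunsmith also messaging the pawn.
; A FlipFlop plays the HUD's key-tip animation forward and in reverse.
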(event EventBeginPlay
  (CameraFades|StartCameraFade :self (Variables|Default|GetPlayerCameraManager) :FromAlpha 1.0 :Duration 5.0))

(event EventTick
  (params (DeltaSeconds :type Float%20%28single-precision%29)))

(event EventPossess
  (params (PossessedPawn :type Pawn%20Object%20Reference))
  (bind _returnvalue (UserInterface|CreateWidget "/Game/Blueprint/UMG/W_PlayerMain.W_PlayerMain_C"))
  (bind _output_get (Variables|Default|SetPlayerMainUI _returnvalue))
  (UserInterface|Viewport|AddtoViewport _output_get 0))

(event EventUnPossess
  (params (UnpossessedPawn :type Pawn%20Object%20Reference))
  (bind _playermainui (Variables|Default|GetPlayerMainUI)
    (:then
      (Widget|RemovefromParent _playermainui)
      (Variables|Default|SetPlayerMainUI 0))
    (:else)))

(event Input|ActionEvents|InputActionToggleWeaponBag
  (params (Key :type Key%20Structure :default "None"))
  (:Pressed
    (bind _weaponbagui (Variables|Default|GetWeaponBagUI)
      (:then
        (Widget|RemovefromParent _weaponbagui)
        (Variables|Default|SetWeaponBagUI 0)
        (CallFunction|GameOnly))
      (:else
        (bind _returnvalue (UserInterface|CreateWidget "/Game/Blueprint/UMG/EasyWeaponBag/W_Bag.W_Bag_C"))
        (bind _output_get (Variables|Default|SetWeaponBagUI _returnvalue))
        (UserInterface|Viewport|AddtoViewport _output_get 0)
        ;[1 1 1] Comment
        (CallFunction|GameandUIInput)))))

(event Input|ActionEvents|InputActionInputTip
  (params (Key :type Key%20Structure :default "None"))
  (:Pressed
    (Utilities|FlowControl|FlipFlop
      (:A
        (bind _playermainui (Variables|Default|GetPlayerMainUI)
          (:then
            (Class|UserWidget|PlayAnimationForward _playermainui (Variables|/Game/Blueprint/UMG/W_PlayerMain.W_PlayerMain_C|GetInputKeyTipAnim _playermainui) 1.0 false))
          (:else)))
      (:B
        (bind _playermainui_2 (Variables|Default|GetPlayerMainUI)
          (:then
            (Class|UserWidget|PlayAnimationReverse _playermainui_2 (Variables|/Game/Blueprint/UMG/W_PlayerMain.W_PlayerMain_C|GetInputKeyTipAnim _playermainui_2) 1.0 false))
          (:else))))))

(event Input|ActionEvents|InputActionAttachment
  (params (Key :type Key%20Structure :default "None"))
  (:Pressed
    (bind _gunsmithui (Variables|Default|GetGunsmithUI)
      (:then
        (Widget|RemovefromParent _gunsmithui)
        (Variables|Default|SetGunsmithUI 0)
        (CallFunction|GameOnly)
        (Class|IPlayerAttrs|SwitchOutGunsmith(Message) (Pawn|GetControlledPawn)))
      (:else
        (bind _returnvalue (UserInterface|CreateWidget "/Game/Blueprint/UMG/Attachment/W_Gunsmith.W_Gunsmith_C"))
        (bind _output_get (Variables|Default|SetGunsmithUI _returnvalue))
        (UserInterface|Viewport|AddtoViewport _output_get 0)
        (CallFunction|GameandUIInput)
        (Class|IPlayerAttrs|SwitchIntoGunsmith(Message) (Pawn|GetControlledPawn))))))

(fn ConstructionScript)

(fn GameandUIInput
  (Input|SetInputModeGameandUI self 0 "DoNotLock" true)
  (Variables|Default|SetbShowMouseCursor true)
  (Utilities|SetInputMode "NewEnumerator1"))

(fn GameOnly
  (Input|SetInputModeGameOnly self)
  (Variables|Default|SetbShowMouseCursor false)
  (Utilities|SetInputMode "NewEnumerator2"))
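; Base weapon Blueprint that provides pickup, ammo state, attachments and detection highlighting.
; On BeginPlay it derives a row name from its display name, then uses DataTable rows to set meshes, anim class, ammo and the fire component.
; Attachments swap component meshes, match against weapon data, update the owner's props and scope offset, and are stored.
; Magazine material slots show remaining rounds, while detection toggles custom depth and the weapon tip widget.
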(event EventBeginPlay
  (CallFunction|Initialize))

(event EventSetAmmos
  (params (CurrentAmmo :type Integer) (MaxAmmo :type Integer))
  (Variables|Attr|Ammo|SetCurrent%20Ammo CurrentAmmo)
  (Variables|Attr|Ammo|SetMax%20Ammo MaxAmmo))

(event EventTick
  (params (DeltaSeconds :type Float%20%28single-precision%29)))

(event EventSetSlideBack
  (params (InVal :type Boolean))
  (Variables|Attr|SetbSlideBack InVal))

(event EventCallUpdateAmmoVisible
  (CallFunction|AmmoCalculate)
  (CallFunction|UpdateMagAmmoVisible))

(event EventOnDetected
  (params (Owner :type Pawn%20Object%20Reference) (Active :type Boolean))
  (Rendering|SetRenderCustomDepth (Variables|Default|GetWeaponMesh) Active)
  (Rendering|SetRenderCustomDepth (Variables|Default|GetDefaultScope) Active)
  (Rendering|SetRenderCustomDepth (Variables|Default|GetMag) Active)
  (Rendering|SetRenderCustomDepth (Variables|Default|GetScope) Active)
  (Rendering|SetRenderCustomDepth (Variables|Default|GetLaser) Active)
  (Rendering|SetRenderCustomDepth (Variables|Default|GetGrip) Active)
  (Rendering|SetRenderCustomDepth (Variables|Default|GetSilencer) Active)
  ;[1 0.2944 0.3942] 更新互动提示武器信息UI
  (Rendering|SetVisibility (Variables|Default|GetWeaponTipUI) Active false)
  (bind _values (Utilities|Map|Values (Variables|Default|GetEquippedAttachment)))
  (for _array_element _values
    (Class|IUI|CallUpdateInteractTip(Message) (UserInterface|GetWidget (Variables|Default|GetWeaponTipUI)) (Variables|Attr|GetWeaponName) (.Icons (Utilities|Struct|BreakS_WeaponAttrs (Variables|Default|GetWeapon%20Attr))) _array_element)))

(event EventPickUp
  (params (Owner :type Pawn%20Object%20Reference))
  (Class|IPlayerAttrs|SetCurrentWeapon(Message) Owner self))

(event EventSetAttachment
  (params (AttachmentProp :type S%20Attachment%20Props%20Structure))
  (bind (_attachmentname _attachmenttype _attachmentmesh) (Utilities|Struct|BreakS_AttachmentProps AttachmentProp))
  (Components|StaticMesh|SetStaticMesh (Utilities|Select :Index _attachmenttype :NewEnumerator0 0 :NewEnumerator1 (Variables|Default|GetScope) :NewEnumerator2 (Variables|Default|GetSilencer) :NewEnumerator3 (Variables|Default|GetLaser) :NewEnumerator4 (Variables|Default|GetGrip)) _attachmentmesh)
  (Utilities|FlowControl|Sequence
    (:then_0
      (bind (_returnvalue _attachmentprop) (Utilities|CallUpdateAttachmentUI _attachmentname _attachmenttype)
        (:LoopBody
          (if _returnvalue
            (CallFunction|UpdateAimOffset _attachmentprop)))))
    (:then_1
      (bind (_returnvalue_2 _attachmentprop_2) (Utilities|CallUpdateAttachmentUI _attachmentname _attachmenttype)
        (:LoopBody
          (if _returnvalue_2
            (Class|IPlayerAttrs|CallonUpdateAttachmentProps(Message) (Components|GetOwner) _attachmentprop_2)))))
    (:then_2
      ;[0 1 0.0583] 将已经配好的配件存储起来（配件的集合要有默认值）
      (bind (_returnvalue_3 _attachmentprop_3) (Utilities|CallUpdateAttachmentUI _attachmentname _attachmenttype)
        (:LoopBody
          (if _returnvalue_3
            (Utilities|Map|Add (Variables|Default|GetEquippedAttachment) _attachmenttype _attachmentprop_3)))))))

(fn ConstructionScript)

(fn Initialize
  (bind _self self)
  (bind _returnvalue (Utilities|GetDisplayName _self))
  (Variables|Attr|SetWeaponName (Utilities|String|StringToName (Utilities|String|GetSubstring _returnvalue 3 (- (Utilities|String|Len _returnvalue) 3))))
  (CallFunction|SetWeaponBodyMesh)
  (bind _weaponanims (CallFunction|GetWeaponAnims))
  (Class|SkeletalMeshComponent|SetAnimClass (Variables|Default|GetWeaponMesh) (.WeaponAnimInstance (Utilities|Struct|BreakS_WeaponAnims _weaponanims)))
  (bind _weaponattr (CallFunction|GetWeaponAttrs))
  (Variables|Attr|Ammo|SetCurrent%20Ammo (.StandardAmmo (Utilities|Struct|BreakS_WeaponAttrs _weaponattr)))
  (Variables|Attr|Ammo|SetMax%20Ammo (.MaxAmmo (Utilities|Struct|BreakS_WeaponAttrs _weaponattr)))
  (Default|Initialize (Variables|Default|GetWeaponSystemComp) (.FireDuration (Utilities|Struct|BreakS_WeaponAttrs _weaponattr)) (.bAutoFire (Utilities|Struct|BreakS_WeaponAttrs _weaponattr))))

(fn SetWeaponBodyMesh
  (bind _weaponattr (CallFunction|GetWeaponAttrs))
  (Variables|Default|SetWeapon%20Attr _weaponattr)
  (Class|SkinnedMeshComponent|SetSkeletalMesh (Variables|Default|GetWeaponMesh) (.WeaponBodyMesh (Utilities|Struct|BreakS_WeaponAttrs _weaponattr)) true)
  (Components|StaticMesh|SetStaticMesh (Variables|Default|GetDefaultScope) (.DefaultScopeMesh (Utilities|Struct|BreakS_WeaponAttrs _weaponattr)))
  (Components|StaticMesh|SetStaticMesh (Variables|Default|GetMag) (.MagMesh (Utilities|Struct|BreakS_MagzineSettings (.MagzineSettings (Utilities|Struct|BreakS_WeaponAttrs _weaponattr))))))

(fn AmmoCalculate
  (bind _mag (Variables|Default|GetMag))
  (bind _weapon_attr (Variables|Default|GetWeapon%20Attr))
  (bind (_standardammo _firesuppressedeffect _magzinesettings) (Utilities|Struct|BreakS_WeaponAttrs _weapon_attr))
  (bind _returnvalue (Rendering|Material|GetNumMaterials _mag))
  (bind _visibleammoindex (Utilities|Struct|BreakS_MagzineSettings _magzinesettings))
  (bind _returnvalue_2 (- _returnvalue _visibleammoindex))
  (Variables|Default|SetCalculation (+ (- _returnvalue_2 (Math|Float|Ceil (* _returnvalue_2 (/ (Math|Conversions|ToFloat(Integer) (Variables|Attr|Ammo|GetCurrent%20Ammo)) (Math|Conversions|ToFloat(Integer) _standardammo))))) (Utilities|Struct|BreakS_MagzineSettings (.MagzineSettings (Utilities|Struct|BreakS_WeaponAttrs (Variables|Default|GetWeapon%20Attr)))))))

(fn UpdateMagAmmoVisible
  (bind _weapon_attr (Variables|Default|GetWeapon%20Attr))
  (bind _magzinesettings (Utilities|Struct|BreakS_WeaponAttrs _weapon_attr))
  (bind (_magmesh _visibleammoindex _defaultammomat _invisibleammomat) (Utilities|Struct|BreakS_MagzineSettings _magzinesettings))
  (for _index (range (Utilities|Struct|BreakS_MagzineSettings (.MagzineSettings (Utilities|Struct|BreakS_WeaponAttrs (Variables|Default|GetWeapon%20Attr)))) (Rendering|Material|GetNumMaterials (Variables|Default|GetMag)))
    (if (< _index (Variables|Default|GetCalculation))
      (Rendering|Material|SetMaterial (Variables|Default|GetMag) _index _invisibleammomat)
      (else
        (Rendering|Material|SetMaterial (Variables|Default|GetMag) _index _defaultammomat)))))

(fn UpdateAimOffset
  (params (AttachmentProps :type S%20Attachment%20Props%20Structure))
  (bind (_attachmenttype _attachmentoffset) (Utilities|Struct|BreakS_AttachmentProps AttachmentProps))
  (if (Utilities|Enum|Equal(Enum) _attachmenttype "NewEnumerator1")
    (Class|IPlayerAttrs|SetWeaponScopeOffset(Message) (Components|GetOwner) _attachmentoffset)))

(fn GetAmmos
  (bind _weaponattr (CallFunction|GetWeaponAttrs))
  (return (Variables|Attr|Ammo|GetCurrent%20Ammo) (Variables|Attr|Ammo|GetMax%20Ammo) (.StandardAmmo (Utilities|Struct|BreakS_WeaponAttrs _weaponattr))))

(fn GetSlideBack
  (return (Variables|Attr|GetbSlideBack)))

(fn GetSocketNames
  (return (Variables|Default|GetSocketNames)))

(fn GetWeaponAnims
  (bind _weaponanimsdt (Variables|DataTable|GetWeaponAnimsDT)
    (:then
      (bind _returnvalue (Utilities|GetDataTableRow _weaponanimsdt (Variables|Attr|GetWeaponName))
        (:then
          (return _returnvalue))))
    (:else)))

(fn GetWeaponAttrs
  (bind _returnvalue (Utilities|GetDataTableRow (Variables|DataTable|GetWeaponAttrsDT) (Variables|Attr|GetWeaponName))
    (:then
      (return _returnvalue))))

(fn GetWeaponMesh
  (bind _weaponmesh (Variables|Default|GetWeaponMesh)
    (:then
      (return _weaponmesh))
    (:else)))

(fn GetWeaponName
  (return (Variables|Attr|GetWeaponName)))
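; BP_Grenade is a grenade projectile that explodes when the actor is destroyed.
; On BeginPlay it runs the parent logic, then unbinds all hit events from its collision component, so impacts do not trigger those handlers.
; On Destroyed it fires a radial force impulse, spawns an explosion emitter and a temporary decal at its location, and plays a distance-based world camera shake.
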(event EventBeginPlay
  (|CallParentFunction)
  (EventDispatchers|UnbindallEventsfromOnComponentHit (Variables|Default|GetProjectileCollision)))

(event EventDestroyed
  (Class|RadialForceComponent|FireImpulse (Variables|Default|GetRadialForce))
  (Effects|SpawnEmitteratLocation "/Game/LowPolyShooterPack/Art/Effects/Particles/PS_EXP.PS_EXP" (Transformation|GetActorLocation) (Transformation|GetActorRotation))
  (Rendering|Decal|SpawnDecalatLocation "/Game/LowPolyShooterPack/Art/Effects/Materials/MI_Decal_Explosion_001.MI_Decal_Explosion_001" "250.000000,250.000000,250.000000" (Transformation|GetActorLocation) (Transformation|GetActorRotation) 8.0)
  (Camera|PlayWorldCameraShake "/Game/Blueprint/CameraShake/CS_Explode.CS_Explode_C" (Transformation|GetActorLocation) 8e+02 1.2e+03))

(fn ConstructionScript
  (|CallParentFunction))
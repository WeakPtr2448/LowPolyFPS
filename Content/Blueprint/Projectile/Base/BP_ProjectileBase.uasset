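; Base projectile Blueprint that is launched along a given direction and speed and produces surface-specific impacts.
; On collision hit, the physical surface type's name selects a data table row supplying the particle, decal and sound.
; HitEffect spawns the emitter and attached decal along the hit normal and applies a mass-independent impulse to physics-simulating components.
; The actor destroys itself only when a matching row is found.
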(event OnComponentHit(ProjectileCollision)
  (params (HitComponent :type Primitive%20Component%20Object%20Reference) (OtherActor :type Actor%20Object%20Reference) (OtherComp :type Primitive%20Component%20Object%20Reference) (NormalImpulse :type Vector :default "0, 0, 0") (Hit :type Hit%20Result%20Structure%20%28by%20ref%29))
  (bind (_bblockinghit _binitialoverlap _time _distance _location _impactpoint _normal _impactnormal _physmat _hitactor _hitcomponent _hitbonename) (Collision|BreakHitResult Hit))
  (bind _returnvalue (Utilities|GetDataTableRow (Variables|Default|GetSurfaceDT) (Utilities|String|StringToName (Utilities|String|EnumtoString (Collision|GetSurfaceType Hit))))
    (:then
      (CallFunction|HitEffect (.HitEffect (Utilities|Struct|BreakS_Surface _returnvalue)) (.HitDecal (Utilities|Struct|BreakS_Surface _returnvalue)) _hitcomponent _normal _impactpoint _hitbonename)
      (Audio|PlaySoundatLocation (.HitSound (Utilities|Struct|BreakS_Surface _returnvalue)) _impactpoint "0, 0, 0" 1.0 1.0 0.0 "/Game/Blueprint/Attenuation/SA_Impact.SA_Impact" 0 0)
      (Actor|DestroyActor))))

(event Custom|Initialize
  (params (LaunchDir :type Vector) (Speed :type Float%20%28single-precision%29))
  (Variables|/Script/Engine.MovementComponent|SetVelocity (Variables|Default|GetProjectileMovement) (* LaunchDir Speed)))

(fn ConstructionScript)

(fn HitEffect
  (params (EmitterTemplate :type Particle%20System%20Object%20Reference) (DecalMaterial :type Material%20Interface%20Object%20Reference) (HitComponent :type Scene%20Component%20Object%20Reference) (Normal :type Vector) (ImpactPoint :type Vector) (BoneName :type Name))
  (bind _returnvalue (Math|Conversions|RotationFromXVector Normal))
  (Effects|SpawnEmitteratLocation EmitterTemplate ImpactPoint _returnvalue)
  (Class|GameplayStatics|SpawnDecalAttached DecalMaterial "2.000000,2.000000,2.000000" HitComponent "None" ImpactPoint _returnvalue "KeepWorldPosition" 2e+01)
  (bind _asprimitive_component (Utilities|Casting|CastToPrimitiveComponent HitComponent))
  (if (Physics|IsSimulatingPhysics _asprimitive_component "None")
    (Physics|AddImpulse _asprimitive_component (* (Math|Vector|Normalize (Transformation|GetVelocity)) 3e+02) BoneName true)))
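; BP_Eject is a projectile-derived actor for an ejected physics object that is thrown by an impulse.
; On BeginPlay it runs the parent logic, turns on physics simulation for its mesh and unbinds all hit events from the collision component.
; LaunchEject applies the given vector to the mesh as a velocity-change impulse, so mass is ignored; nothing in this graph actively calls it.
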(event EventBeginPlay
  (|CallParentFunction)
  (Physics|SetSimulatePhysics (Variables|Default|GetProjectileMesh) true)
  (EventDispatchers|UnbindallEventsfromOnComponentHit (Variables|Default|GetProjectileCollision)))

(event Collision|EventActorBeginOverlap
  (params (OtherActor :type Actor%20Object%20Reference)))

(event EventTick
  (params (DeltaSeconds :type Float%20%28single-precision%29)))

(fn ConstructionScript
  (|CallParentFunction))

(fn LaunchEject
  (params (Force :type Vector))
  (Physics|AddImpulse (Variables|Default|GetProjectileMesh) Force "None" true))